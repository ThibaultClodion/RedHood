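; Base Blueprint for 2D PaperZD characters, providing a shared melee attack and hit reaction.
; AttackBoxTrace sweeps an oriented box between two marker components and calls GetHit on any BP_CharacterBase it strikes first.
; GetHit plays the hit-react animation override and disables player input; SetInputEnabled can also restore it.
; Attack and hit animations play as PaperZD overrides, and no damage value is applied.
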(fn `AttackBoxTrace`
  (bind _outhit (`KismetSystemLibrary.BoxTraceSingleForObjects` (`SceneComponent.K2_GetComponentLocation` (`self.BoxTraceStart`)) (`SceneComponent.K2_GetComponentLocation` (`self.BoxTraceEnd`)) (`self.TraceExtent`) (`self.BoxRotation`) (`self.TraceObjectTypes`)))
  (bind _asbp_character_base (cast `/Game/Blueprints/Characters/BP_CharacterBase` (`.HitActor` (`GameplayStatics.BreakHitResult` _outhit))))
  (`self.GetHit` _asbp_character_base))

(fn `GetHit`
  (`self.PlayHitReactAnimation`)
  (`self.SetInputEnabled` false))

(fn `PlayAttackAnim`
  (`PaperZDAnimInstance.K2_PlayAnimationOverride` (`PaperZDAnimationComponent.AnimInstance` (`self.PaperZDAnimation`)) (`self.AttackAnimSequence`) "DefaultSlot" 1.0 0.0))

(fn `PlayHitReactAnimation`
  (`PaperZDAnimInstance.K2_PlayAnimationOverride` (`PaperZDAnimationComponent.AnimInstance` (`self.PaperZDAnimation`)) (`self.HitReactAnimSequence`) "DefaultSlot" 1.0 0.0))

(fn `SetInputEnabled`
  (params (Enabled :type Boolean))
  (bind _asplayer_controller (cast `PlayerController` (`self.GetController`) :!pure true))
  (if Enabled
    (`self.EnableInput` _asplayer_controller)
    (else
      (`self.DisableInput` _asplayer_controller))))

(fn `UserConstructionScript`)